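; BTL player character with Enhanced Input forward-axis movement and a buffered two-hit melee combo, randomly picked from two variants.
; Attack plays montages looked up by combo and step name, while presses mid-attack are saved for AttackCombo to chain or end.
; The opening hit sphere-traces for an enemy, then Motion Warping snaps attacks to its front, back, left or right point, facing it.
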(event Custom|Attack
  (if (Variables|Default|GetCanAttack?)
    (if (Variables|Default|GetIsAttacking?)
      (Variables|Default|SetSaveAttack true)
      (else
        (Variables|Default|SetIsAttacking? true)
        (Variables|Default|SetCombsNumber (Math|Random|RandomIntegerinRange 1 2))
        (switch int (Variables|Default|GetAttackCounter)
          (:0
            (bind _array_element (CallFunction|FindAttackMontage (Variables|Default|GetCombsNumber) 1))
            (CallFunction|UpdateMotionWarping false _array_element)
            (Utilities|FlowControl|DoOnce false :!label _label
              (:Completed
                (Utilities|FlowControl|Delay 0.1)
                (Animation|Montage|PlayMontage (Variables|Character|GetMesh) _array_element
                  (:then
                    (Variables|Default|SetAttackCounter 1)
                    (goto _label Reset))))))
          (:1
            (bind _array_element_2 (CallFunction|FindAttackMontage (Variables|Default|GetCombsNumber) 2))
            (CallFunction|UpdateMotionWarping true _array_element_2)
            (Utilities|FlowControl|DoOnce false :!label _label_2
              (:Completed
                (Utilities|FlowControl|Delay 0.1)
                (Animation|Montage|PlayMontage (Variables|Character|GetMesh) _array_element_2
                  (:then
                    (Variables|Default|SetAttackCounter 0)
                    (goto _label_2 Reset)))))))))))

(event Custom|Attack%20Combo
  (if (Variables|Default|GetSaveAttack)
    (Variables|Default|SetSaveAttack false)
    (switch int (Variables|Default|GetAttackCounter)
      (:0
        (bind _array_element (CallFunction|FindAttackMontage (Variables|Default|GetCombsNumber) 1))
        (CallFunction|UpdateMotionWarping false _array_element)
        (Utilities|FlowControl|DoOnce false :!label _label
          (:Completed
            (Utilities|FlowControl|Delay 0.1)
            (Animation|Montage|PlayMontage (Variables|Character|GetMesh) _array_element
              (:then
                (Variables|Default|SetAttackCounter 1)
                (goto _label Reset))))))
      (:1
        (bind _array_element_2 (CallFunction|FindAttackMontage (Variables|Default|GetCombsNumber) 2))
        (CallFunction|UpdateMotionWarping true _array_element_2)
        (Utilities|FlowControl|DoOnce false :!label _label_2
          (:Completed
            (Utilities|FlowControl|Delay 0.1)
            (Animation|Montage|PlayMontage (Variables|Character|GetMesh) _array_element_2
              (:then
                (Variables|Default|SetAttackCounter 0)
                (goto _label_2 Reset)))))))
    (else
      (CallFunction|ComboEnd))))

(event Custom|Combo%20End
  (Variables|Default|SetAttackCounter 0)
  (Variables|Default|SetIsAttacking? false)
  (Variables|Default|SetEnemy 0)
  (Class|MotionWarpingComponent|RemoveWarpTarget (Variables|Default|GetMotionWarping) "Attack"))

(event Custom|Update%20Motion%20Warping
  (params (Combo :type Boolean) (Anim%20Montage :type Anim%20Montage%20Object%20Reference))
  (bind _arrow1 (Variables|Default|GetArrow1))
  (bind _returnvalue (Transformation|GetWorldLocation _arrow1))
  (if (not Combo)
    (bind (_outhit _returnvalue_2) (Collision|SphereTraceForObjects _returnvalue (+ _returnvalue (* (Math|Vector|GetForwardVector (Transformation|GetWorldRotation _arrow1)) 2e+02)) 9e+01 (Utilities|Array|MakeArray "ObjectTypeQuery3") false 0 "ForDuration"))
    (if _returnvalue_2
      (if (Utilities|DoesObjectImplementInterface (.HitActor (Collision|BreakHitResult _outhit)) "/Game/Blueprints/Character/Interface/BPI_GetEnemy.BPI_GetEnemy_C")
        (bind _enemy (Class|BPIGetEnemy|GetEnemyReference(Message) (.HitActor (Collision|BreakHitResult _outhit))))
        (bind _output_get (Variables|Default|SetEnemy _enemy))
        (bind _e_direction (Default|GetEnemyHitDirection _output_get (Transformation|GetActorLocation)))
        (Utilities|IsValid (Variables|Default|GetEnemy) :!label _label
          (:Is%20Valid
            (Class|MotionWarpingComponent|AddorUpdateWarpTarget (Variables|Default|GetMotionWarping) (Utilities|Struct|MakeMotionWarpingTarget "Attack" (Transformation|GetWorldLocation (Utilities|Select :Index _e_direction :NewEnumerator0 (Variables|/Game/Blueprints/Character/MainEnemy/BP_BTLEnemy.BP_BTLEnemy_C|GetLeft (Variables|Default|GetEnemy)) :NewEnumerator1 (Variables|/Game/Blueprints/Character/MainEnemy/BP_BTLEnemy.BP_BTLEnemy_C|GetRight (Variables|Default|GetEnemy)) :NewEnumerator2 (Variables|/Game/Blueprints/Character/MainEnemy/BP_BTLEnemy.BP_BTLEnemy_C|GetFront (Variables|Default|GetEnemy)) :NewEnumerator3 (Variables|/Game/Blueprints/Character/MainEnemy/BP_BTLEnemy.BP_BTLEnemy_C|GetBack (Variables|Default|GetEnemy)))) (Math|Rotator|FindLookatRotation (Transformation|GetActorLocation) (Transformation|GetActorLocation (Variables|Default|GetEnemy))) 0 "None" false))))))
    (else
      (goto _label))))

(event Input|EnhancedActionEvents|EnhancedInputActionIA_Move
  (params (ActionValue :type Float%20%28double-precision%29) (ElapsedSeconds :type Float%20%28double-precision%29) (TriggeredSeconds :type Float%20%28double-precision%29) (InputAction :type Input%20Action%20Object%20Reference :default "/Game/Blueprints/Input/InputAction/IA_Move.IA_Move"))
  (Pawn|Input|AddMovementInput (Transformation|GetActorForwardVector) ActionValue false))

(event Input|EnhancedActionEvents|EnhancedInputActionIA_Attack
  (params (ActionValue :type Boolean) (ElapsedSeconds :type Float%20%28double-precision%29) (TriggeredSeconds :type Float%20%28double-precision%29) (InputAction :type Input%20Action%20Object%20Reference :default "/Game/Blueprints/Input/InputAction/IA_Attack.IA_Attack"))
  (:Started
    (CallFunction|Attack)))

(event EventBeginPlay
  (Input|AddMappingContext (PlayerController|LocalPlayerSubsystems|GetEnhancedInputLocalPlayerSubsystem (Game|GetPlayerController 0)) "/Game/Blueprints/Input/IMC_BTLContext.IMC_BTLContext" 0 "(bIgnoreAllPressedKeysUntilRelease=True,bForceImmediately=False,bNotifyUserSettings=False)"))

(fn ConstructionScript
  (|CallParentFunction))

(fn FindAttackMontage
  (params (Combo :type Integer) (Num :type Integer))
  (bind _keys (Utilities|Map|Keys (Variables|Default|GetAnimMontage)))
  (for _array_element _keys
    (if (Utilities|Enum|Equal(Enum) (Utilities|Struct|BreakS_AnimMontage (.Value (Utilities|Map|Find (Variables|Default|GetAnimMontage) _array_element))) (Utilities|String|Append (Utilities|String|Append "Combo" (Utilities|String|ToString(Integer) Combo)) (Utilities|String|Append "Num" (Utilities|String|ToString(Integer) Num))))
      (return _array_element))))