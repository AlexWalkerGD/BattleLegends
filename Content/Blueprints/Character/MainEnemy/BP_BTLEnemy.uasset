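; BP_BTLEnemy is an enemy character Blueprint that works out which side a hit landed on.
; GetEnemyHitDirection measures the hit location against the Right, Back, Left and Front direction components, then maps the nearest one within a starting distance threshold to a direction enum.
; GetEnemyReference returns the enemy itself.
; The event graph holds only disabled default events, and construction just calls the parent.
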(event EventBeginPlay
  (|CallParentFunction) ; This node is disabled and will not be called.\nDrag off pins to build functionality.
)

(event Collision|EventActorBeginOverlap
  (params (OtherActor :type Actor%20Object%20Reference))
  (|CallParentFunction OtherActor) ; This node is disabled and will not be called.\nDrag off pins to build functionality.
)

(event EventTick
  (params (DeltaSeconds :type Float%20%28single-precision%29))
  (|CallParentFunction DeltaSeconds) ; This node is disabled and will not be called.\nDrag off pins to build functionality.
)

(fn ConstructionScript
  (|CallParentFunction))

(fn GetEnemyHitDirection
  (params (Hit%20Location :type Vector))
  (Utilities|FlowControl|DoOnce false :!label _label
    (:Completed
      (LocalVariables|SetGetNearestArrow 5e+02)
      (for (_array_element _array_index) (Utilities|Array|MakeArray (Math|Vector|Distance(Vector) Hit%20Location (Transformation|GetWorldLocation (Variables|Default|GetRight))) (Math|Vector|Distance(Vector) Hit%20Location (Transformation|GetWorldLocation (Variables|Default|GetBack))) (Math|Vector|Distance(Vector) Hit%20Location (Transformation|GetWorldLocation (Variables|Default|GetLeft))) (Math|Vector|Distance(Vector) Hit%20Location (Transformation|GetWorldLocation (Variables|Default|GetFront))))
        (Math|Float|CompareFloat _array_element (LocalVariables|GetGetNearestArrow)
          (:<
            (LocalVariables|SetGetNearestArrow _array_element)
            (LocalVariables|SetGetNearestIndex _array_index))))
      (Utilities|FlowControl|Sequence
        (:then_0
          (goto _label Reset))
        (:then_1
          (return (Utilities|Select :Index (LocalVariables|GetGetNearestIndex) :Option%200 "NewEnumerator1" :Option%201 "NewEnumerator3" :Option%202 "NewEnumerator0" :Option%203 "NewEnumerator2")))))))

(fn GetEnemyReference
  (return self))